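; Construction-script placement actor that lines up book actors in a row along local X as child actor components.
; Books come from BooksToStack, in order or randomized, either once per entry or looped until the row passes LoopLength, with a capped iteration count.
; Each BP_MasterBook child receives the stacker's size and random-size settings, then its resized collision box width plus ExtraSpacing sets the next book's offset.
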(event Custom|SpawnBooks
  (bind _bookstostack (Variables|Default|GetBooksToStack))
  (if (> (Utilities|Array|Length (Variables|Default|GetBooksToStack)) 0)
    (for _index (range 0 (select (Variables|Default|GetLoop?) 500 (Utilities|Array|LastIndex (Variables|Default|GetBooksToStack))))
      (if (select (Variables|Default|GetLoop?) (<= (Variables|Default|GetRowLength) (Variables|Default|GetLoopLength)) true)
        (bind _returnvalue (AddComponent|AddChildActorComponent false (Math|Transform|MakeTransform (Math|Vector|MakeVector (Variables|Default|GetRowLength) 0.0 0.0) (Math|Rotator|MakeRotator 0.0 (Variables|Default|GetYRotation) 0.0) "1.000000,1.000000,1.000000")))
        (ChildActorComponent|SetChildActorClass _returnvalue (select (Variables|Default|GetRandomizeBooks?) (Utilities|Array|Get(acopy) _bookstostack (Math|Random|RandomIntegerinRange 0 (Utilities|Array|LastIndex _bookstostack))) (Utilities|Array|Get(acopy) (Variables|Default|GetBooksToStack) (Variables|Default|GetCurrentIndex))))
        (bind _asbp_master_book (Utilities|Casting|CastToBP_MasterBook (Variables|/Script/Engine.ChildActorComponent|GetChildActor _returnvalue)))
        (Variables|/Game/InteractiveBook/Blueprints/BP_MasterBook.BP_MasterBook_C|SetBookSize _asbp_master_book (Variables|Default|GetBookSize))
        (Variables|/Game/InteractiveBook/Blueprints/BP_MasterBook.BP_MasterBook_C|SetBookRandomSize? _asbp_master_book (Variables|Default|GetBookRandomSize?))
        (Variables|/Game/InteractiveBook/Blueprints/BP_MasterBook.BP_MasterBook_C|SetBookRandomSizeMin _asbp_master_book (Variables|Default|GetBookRandomSizeMin))
        (Variables|/Game/InteractiveBook/Blueprints/BP_MasterBook.BP_MasterBook_C|SetBookRandomSizeMax _asbp_master_book (Variables|Default|GetBookRandomSizeMax))
        (Default|SetBookSize _asbp_master_book)
        (Variables|Default|SetRowLength (+ (Variables|Default|GetRowLength) (+ (* (.x (Components|Box|GetScaledBoxExtent (Variables|/Game/InteractiveBook/Blueprints/BP_MasterBook.BP_MasterBook_C|GetBookCollision _asbp_master_book))) 2.0) (Variables|Default|GetExtraSpacing))))
        (if (== (Variables|Default|GetCurrentIndex) (Utilities|Array|LastIndex (Variables|Default|GetBooksToStack)))
          (Variables|Default|SetCurrentIndex 0)
          (else
            (Math|Integer|IncrementInt (Variables|Default|GetCurrentIndex))))))))

(fn ConstructionScript
  (CallFunction|SpawnBooks))